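; Lobby player controller that shows the lobby menu and lets a client trigger the start of the game.
; On BeginPlay it creates the lobby widget if needed, adds it to the viewport and switches to cursor-visible UI-only input.
; It also caches the game instance as ServerInfo.
; ClientStartGame calls TravelServer on that instance when CanStart is true.
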(event Custom|Client%20Start%20Game
  (if (Variables|Default|GetbCanStart)
    (Default|TravelServer (Variables|Default|GetRef_ServerInfo))))

(event EventBeginPlay
  (bind _returnvalue (Game|GetPlayerController 0))
  (Utilities|IsValid (stale _returnvalue_2)
    (:Is%20Valid
      _)
    (:Is%20Not%20Valid
      (bind _returnvalue_2 (UserInterface|CreateWidget "/Game/MainMenu/WBP_LobbyMenu.WBP_LobbyMenu_C" _returnvalue))))
  (UserInterface|Viewport|AddtoViewport _returnvalue_2 0)
  (Variables|/Script/Engine.PlayerController|SetbShowMouseCursor _returnvalue true)
  (Input|SetInputModeUIOnly _returnvalue 0 "DoNotLock")
  (bind _asserver_info (Utilities|Casting|CastToServerInfo (Game|GetGameInstance)))
  (Variables|Default|SetRef_ServerInfo _asserver_info))

(event EventTick
  (params (DeltaSeconds :type Float%20%28single-precision%29)))

(fn ConstructionScript)