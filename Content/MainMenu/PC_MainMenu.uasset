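; PC_MainMenu is the main menu player controller that shows the menu and forwards session requests.
; On BeginPlay it caches the ServerInfo game instance, then creates WBP_MainMenu if needed, adds it to the viewport and switches to mouse-driven, UI-only input.
; Its ClientHostSession and ClientJoinSession events pass host and join calls through to ServerInfo.
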(event Custom|Client%20Host%20Session
  (Default|HostSession (Variables|Default|GetRef_ServerInfo)))

(event Custom|Client%20Join%20Session
  (Default|JoinSession (Variables|Default|GetRef_ServerInfo)))

(event EventBeginPlay
  (bind _returnvalue (Game|GetPlayerController 0))
  (bind _asserver_info (Utilities|Casting|CastToServerInfo (Game|GetGameInstance)))
  (Variables|Default|SetRef_ServerInfo _asserver_info)
  (Utilities|IsValid (stale _returnvalue_2)
    (:Is%20Valid
      _)
    (:Is%20Not%20Valid
      (bind _returnvalue_2 (UserInterface|CreateWidget "/Game/MainMenu/WBP_MainMenu.WBP_MainMenu_C" (Game|GetPlayerController 0)))))
  (UserInterface|Viewport|AddtoViewport _returnvalue_2 0)
  (Variables|/Script/Engine.PlayerController|SetbShowMouseCursor _returnvalue true)
  (Input|SetInputModeUIOnly _returnvalue _returnvalue_2 "DoNotLock"))

(fn ConstructionScript)