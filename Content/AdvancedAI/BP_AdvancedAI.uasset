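; BP_AdvancedAI is an AI character that runs the BT_AdvancedAI behavior tree and can drop a powerup when it dies.
; When its health component first reports zero health or less, ServerGenRanNum rolls a random number from 0 to 9.
; The RandomNumber RepNotify spawns a health powerup on 0 or a speed powerup on 5 at the actor's location, with no authority check.
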(event OnHealthChanged(HealthComp)
  (params (InHealthComp :type S%20Health%20Component%20Object%20Reference) (Health :type Float%20%28single-precision%29) (HealthDelta :type Float%20%28single-precision%29) (DamageType :type Damage%20Type%20Object%20Reference) (InstigatedBy :type Controller%20Object%20Reference) (DamageCauser :type Actor%20Object%20Reference))
  (if (and (not (Variables|Default|GetbHasGeneratedNumber)) (<= Health 0.0))
    (CallFunction|ServerGenRanNum)))

(event Custom|ServerGenRanNum
  (Variables|Default|SetbHasGeneratedNumber true)
  (Variables|Default|SetRandomNumber (Math|Random|RandomInteger 10)))

(event Custom|SpawnSpeedPowerup
  (Game|SpawnActorfromClass "/Game/Powerups/SpeedPowerup/BP_SpeedPowerup.BP_SpeedPowerup_C" (Math|Conversions|ToTransform(Vector) (Transformation|GetActorLocation)) "Undefined" 0 0))

(event Custom|SpawnHealthPowerup
  (Game|SpawnActorfromClass "/Game/Powerups/HealthPowerup/BP_HealthPowerup.BP_HealthPowerup_C" (Math|Conversions|ToTransform(Vector) (Transformation|GetActorLocation)) "Undefined" 0 0))

(event EventBeginPlay
  (bind _self self)
  (bind _returnvalue (AI|GetAIController _self))
  (Utilities|IsValid _returnvalue
    (:Is%20Valid
      (AI|RunBehaviorTree _returnvalue "/Game/AdvancedAI/BT_AdvancedAI.BT_AdvancedAI"))))

(fn ConstructionScript)

(fn ServerGenerateNumber)

(fn OnRepRandomNumber
  (switch int (Variables|Default|GetRandomNumber)
    (:0
      (CallFunction|SpawnHealthPowerup))
    (:5
      (CallFunction|SpawnSpeedPowerup))))