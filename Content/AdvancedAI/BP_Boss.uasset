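; BP_Boss is an AI-controlled boss enemy whose default health scales with the current round and which can drop a powerup on death.
; BeginPlay starts the BT_Boss behavior tree, and Tick prints health for debugging.
; At zero health, the capsule ignores Pawn and Camera channels and a one-time random roll runs.
; The RandomNumber RepNotify spawns a health or speed powerup on specific results.
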(event OnHealthChanged(HealthComp)
  (params (InHealthComp :type S%20Health%20Component%20Object%20Reference) (Health :type Float%20%28single-precision%29) (HealthDelta :type Float%20%28single-precision%29) (DamageType :type Damage%20Type%20Object%20Reference) (InstigatedBy :type Controller%20Object%20Reference) (DamageCauser :type Actor%20Object%20Reference))
  (bind _returnvalue (<= Health 0.0))
  (bind _capsulecomponent (Variables|Default|GetCapsuleComponent))
  (if _returnvalue
    (Collision|SetCollisionResponsetoChannel _capsulecomponent "ECC_Pawn" "ECR_Ignore")
    (Collision|SetCollisionResponsetoChannel _capsulecomponent "ECC_Camera" "ECR_Ignore")
    (if (and (not (Variables|Default|GetbHasGeneratedNumber)) _returnvalue)
      (CallFunction|ServerGenRanNum))))

(event Custom|ServerGenRanNum
  (Variables|Default|SetbHasGeneratedNumber true)
  (Variables|Default|SetRandomNumber (Math|Random|RandomInteger 15)))

(event Custom|SpawnSpeedPowerup
  (Game|SpawnActorfromClass "/Game/Powerups/SpeedPowerup/BP_SpeedPowerup.BP_SpeedPowerup_C" (Math|Conversions|ToTransform(Vector) (Transformation|GetActorLocation)) "Undefined" 0 0))

(event Custom|SpawnHealthPowerup
  (Game|SpawnActorfromClass "/Game/Powerups/HealthPowerup/BP_HealthPowerup.BP_HealthPowerup_C" (Math|Conversions|ToTransform(Vector) (Transformation|GetActorLocation)) "Undefined" 0 0))

(event EventBeginPlay
  (bind _self self)
  (bind _returnvalue (AI|GetAIController _self))
  (Utilities|IsValid _returnvalue
    (:Is%20Valid
      (AI|RunBehaviorTree _returnvalue "/Game/AdvancedAI/BT_Boss.BT_Boss"))))

(event EventTick
  (params (DeltaSeconds :type Float%20%28single-precision%29))
  (Development|PrintString (Utilities|String|ToString(Float) (Variables|/Script/Survival.SHealthComponent|GetHealth (Variables|Default|GetHealthComp))) true true "(R=0.000000,G=0.660000,B=1.000000,A=1.000000)" 0.0))

(fn ConstructionScript
  (bind _assgame_state (Utilities|Casting|CastToSGameState (Game|GetGameState)))
  (Variables|/Script/Survival.SHealthComponent|SetDefaultHealth (Variables|Default|GetHealthComp) (Math|Conversions|ToFloat(Integer) (* (Variables|/Script/Survival.SGameState|GetCurrentRound _assgame_state) 300))))

(fn ServerGenerateNumber)

(fn OnRepRandomNumber
  (switch int (Variables|Default|GetRandomNumber)
    (:0
      (CallFunction|SpawnHealthPowerup))
    (:5
      (CallFunction|SpawnSpeedPowerup))))