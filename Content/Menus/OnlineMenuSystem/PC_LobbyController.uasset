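; PC_LobbyController is the player controller for the online lobby, handling menus, character choice, ready state and kicks to the main menu.
; An authority check creates either the host or client screen and routes player list updates to it.
; Character changes respawn and possess a matching lobby pawn, while the chosen class is saved to OnlineGameInstance.
; Possession and ready toggles update PlayerInfo and have LobbyGameMode refresh player lists.
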(event Custom|CreateMenus
  (Networking|SwitchHasAuthority
    (:Authority
      (bind _returnvalue (UserInterface|CreateWidget "/Game/Menus/OnlineMenuSystem/WBP_LobbyHostScreen.WBP_LobbyHostScreen_C"))
      (bind _output_get (Variables|Default|SetLobbyWidget _returnvalue))
      (UserInterface|Viewport|AddtoViewport _output_get 0))
    (:Remote
      (bind _returnvalue_2 (UserInterface|CreateWidget "/Game/Menus/OnlineMenuSystem/WBP_LobbyClientScreen.WBP_LobbyClientScreen_C"))
      (bind _output_get_2 (Variables|Default|SetLobbyWidget _returnvalue_2))
      (UserInterface|Viewport|AddtoViewport _output_get_2 0))))

(event Custom|UpdatePlayerList
  (params (PlayerInfo :type Array%20of%20Player%20Info%20Struct%20Structures))
  (Variables|Default|SetConnected%20Player%20Info PlayerInfo)
  (Networking|SwitchHasAuthority
    (:Authority
      (bind _aswbp_lobby_host_screen (Utilities|Casting|CastToWBP_LobbyHostScreen (Variables|Default|GetLobbyWidget)))
      (Default|UpdatePlayerList _aswbp_lobby_host_screen (Variables|Default|GetConnected%20Player%20Info)))
    (:Remote
      (bind _aswbp_lobby_client_screen (Utilities|Casting|CastToWBP_LobbyClientScreen (Variables|Default|GetLobbyWidget)))
      (Default|UpdatePlayerList _aswbp_lobby_client_screen (Variables|Default|GetConnected%20Player%20Info)))))

(event Custom|SetCharacterClass
  (params (ChosenClass :type BP%20Main%20Character%20Class%20Reference))
  (bind _asonline_game_instance (Utilities|Casting|CastToOnlineGameInstance (Game|GetGameInstance)))
  (Variables|/Game/Menus/OnlineMenuSystem/OnlineGameInstance.OnlineGameInstance_C|SetChosenClass _asonline_game_instance ChosenClass))

(event Custom|SetReadyStatus
  (bind _playerinfo (Variables|Default|GetPlayerInfo))
  (Utilities|Struct|SetmembersinPlayerInfoStruct _playerinfo (not (.IsReady (Utilities|Struct|BreakPlayerInfoStruct _playerinfo))))
  (bind _aslobby_game_mode (Utilities|Casting|CastToLobbyGameMode (Game|GetGameMode)))
  (Default|UpdatePlayerLists _aslobby_game_mode))

(event Custom|KickedFromLobby
  (params (Option :type String))
  (Game|OpenLevel(byObjectReference) "/Game/Menus/OnlineMenuSystem/MainMenu.MainMenu" true Option))

(event Custom|ChangeCharacter
  (params (NewCharacter :type BP%20Main%20Character%20Class%20Reference))
  (bind _returnvalue (Pawn|GetControlledPawn))
  (bind _output_get (Variables|Default|SetSpawnTransform (Transformation|GetActorTransform _returnvalue)))
  (Actor|DestroyActor _returnvalue)
  (if (== NewCharacter "/Game/Blueprints/BP_Support.BP_Support_C")
    (Variables|Default|SetLobbyClass "/Game/Menus/OnlineMenuSystem/BP_SupportLobbyCharacter.BP_SupportLobbyCharacter_C")
    (elif (== NewCharacter "/Game/Blueprints/BP_Tank.BP_Tank_C")
      (Variables|Default|SetLobbyClass "/Game/Menus/OnlineMenuSystem/BP_TankLobbyCharacter.BP_TankLobbyCharacter_C")
      (else
        (Variables|Default|SetLobbyClass "/Game/Menus/OnlineMenuSystem/BP_LobbyCharacter.BP_LobbyCharacter_C"))))
  (bind _aspawn (Utilities|Casting|CastToPawnClass (Variables|Default|GetLobbyClass)))
  (bind _returnvalue_2 (Game|SpawnActorfromClass _aspawn _output_get "Undefined" 0 0))
  (Pawn|Possess _returnvalue_2))

(event EventPossess
  (params (PossessedPawn :type Pawn%20Object%20Reference))
  (Utilities|Struct|SetmembersinPlayerInfoStruct (Variables|Default|GetPlayerInfo) PossessedPawn)
  (bind _aslobby_game_mode (Utilities|Casting|CastToLobbyGameMode (Game|GetGameMode)))
  (Default|UpdatePlayerLists _aslobby_game_mode))

(event EventBeginPlay
  (CallFunction|CreateMenus))

(fn ConstructionScript)