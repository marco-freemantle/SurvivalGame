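; Lobby player controller that shows the lobby menu and starts the match travel.
; On BeginPlay it creates WBP_LobbyMenu if needed, adds it to the viewport with cursor and UI-only input, then caches the ServerInfo game instance and BP_LobbyGameMode.
; ClientStartGame checks CanStart, clears all widgets and calls TravelServer on the cached game mode.
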(event Custom|Client%20Start%20Game
  (if (Variables|Default|GetbCanStart)
    (Viewport|RemoveAllWidgets)
    (Default|TravelServer (Variables|Default|GetRef_LobbyGameMode))))

(event EventBeginPlay
  (bind _returnvalue (Game|GetPlayerController 0))
  (Utilities|IsValid (stale _returnvalue_2)
    (:Is%20Valid
      _)
    (:Is%20Not%20Valid
      (bind _returnvalue_2 (UserInterface|CreateWidget "/Game/Menus/LobbyMenu/WBP_LobbyMenu.WBP_LobbyMenu_C" _returnvalue))))
  (UserInterface|Viewport|AddtoViewport _returnvalue_2 0)
  (Variables|/Script/Engine.PlayerController|SetbShowMouseCursor _returnvalue true)
  (Input|SetInputModeUIOnly _returnvalue 0 "DoNotLock")
  (bind _asserver_info (Utilities|Casting|CastToServerInfo (Game|GetGameInstance)))
  (Variables|Default|SetRef_ServerInfo _asserver_info)
  (bind _asbp_lobby_game_mode (Utilities|Casting|CastToBP_LobbyGameMode (Game|GetGameMode)))
  (Variables|Default|SetRef_LobbyGameMode _asbp_lobby_game_mode))

(fn ConstructionScript)