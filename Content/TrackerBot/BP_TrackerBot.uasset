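; BP_TrackerBot is a tracker bot that can drop a health or speed powerup at its location when its health runs out.
; Tick maps movement speed to the audio component's volume, so the bot gets louder as it moves faster.
; On death, a one-time random roll sets the RepNotify RandomNumber, whose OnRep spawns a powerup on two of the possible results.
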(event OnHealthChanged(HealthComp)
  (params (InHealthComp :type S%20Health%20Component%20Object%20Reference) (Health :type Float%20%28single-precision%29) (HealthDelta :type Float%20%28single-precision%29) (DamageType :type Damage%20Type%20Object%20Reference) (InstigatedBy :type Controller%20Object%20Reference) (DamageCauser :type Actor%20Object%20Reference))
  ;[1 1 1] When health == 0, generate random number on the server and pass to clients. If number meets certain conditions then spawn a powerup
  (if (and (not (Variables|Default|GetbHasGeneratedNumber)) (<= Health 0.0))
    (CallFunction|ServerGenerateNumber)))

(event Custom|SpawnHealthPowerup
  (Game|SpawnActorfromClass "/Game/Powerups/HealthPowerup/BP_HealthPowerup.BP_HealthPowerup_C" (Math|Conversions|ToTransform(Vector) (Transformation|GetActorLocation)) "Undefined" 0 0))

(event Custom|SpawnSpeedPowerup
  (Game|SpawnActorfromClass "/Game/Powerups/SpeedPowerup/BP_SpeedPowerup.BP_SpeedPowerup_C" (Math|Conversions|ToTransform(Vector) (Transformation|GetActorLocation)) "Undefined" 0 0))

(event Custom|ServerGenerateNumber
  ;[1 1 1] Generate random number on the server. Store in rep_notify variable
  (Variables|Default|SetbHasGeneratedNumber true)
  (Variables|Default|SetRandomNumber (Math|Random|RandomInteger 15)))

(event EventTick
  (params (DeltaSeconds :type Float%20%28single-precision%29))
  ;[1 1 1] Set Audio volume based upon velocity
  (Audio|Components|Audio|SetVolumeMultiplier (Variables|Default|GetAudioComp) (Math|Float|MapRangeClamped (Math|Vector|VectorLength (Transformation|GetVelocity)) 1e+01 1e+03 0.1 1.0) :!class /Script/Engine.AudioComponent))

(fn ConstructionScript)

(fn OnRepRandomNumber
  (switch int (Variables|Default|GetRandomNumber)
    (:0
      (CallFunction|SpawnHealthPowerup))
    (:5
      (CallFunction|SpawnSpeedPowerup))))