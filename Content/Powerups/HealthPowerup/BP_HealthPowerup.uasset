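; Health pickup actor that restores a damaged team 0 actor to full health.
; It spins around yaw every tick and destroys itself ten seconds after spawning if left unused.
; On mesh overlap, it checks each overlapping actor's SHealthComponent for team and missing health.
; A valid pickup sets Health to DefaultHealth, plays an attached sound, disables collision, hides and destroys the powerup.
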(event OnComponentBeginOverlap(StaticMesh)
  (params (OverlappedComponent :type Primitive%20Component%20Object%20Reference) (OtherActor :type Actor%20Object%20Reference) (OtherComp :type Primitive%20Component%20Object%20Reference) (OtherBodyIndex :type Integer) (bFromSweep :type Boolean) (SweepResult :type Hit%20Result%20Structure%20%28by%20ref%29))
  (bind _staticmesh (Variables|Default|GetStaticMesh))
  (bind _staticmesh_2 (Variables|Default|GetStaticMesh))
  (Utilities|IsValid _staticmesh
    (:Is%20Valid
      (for _array_element (Collision|GetOverlappingActors _staticmesh 0 :!class /Script/Engine.PrimitiveComponent)
        (Utilities|IsValid _array_element
          (:Is%20Valid
            (Utilities|IsValid (Actor|GetComponentbyClass _array_element "/Script/Survival.SHealthComponent")
              (:Is%20Valid
                (if (== (Variables|/Script/Survival.SHealthComponent|GetTeamNum (Actor|GetComponentbyClass _array_element "/Script/Survival.SHealthComponent")) 0)
                  (if (< (Variables|/Script/Survival.SHealthComponent|GetHealth (Actor|GetComponentbyClass _array_element "/Script/Survival.SHealthComponent")) (Variables|/Script/Survival.SHealthComponent|GetDefaultHealth (Actor|GetComponentbyClass _array_element "/Script/Survival.SHealthComponent")))
                    (Variables|/Script/Survival.SHealthComponent|SetHealth (Actor|GetComponentbyClass _array_element "/Script/Survival.SHealthComponent") (Variables|/Script/Survival.SHealthComponent|GetDefaultHealth (Actor|GetComponentbyClass _array_element "/Script/Survival.SHealthComponent")))
                    (Audio|SpawnSoundAttached "/Game/Powerups/Pickup-Sound_Cue.Pickup-Sound_Cue" _staticmesh_2 "None" "0, 0, 0" "0, 0, 0" "KeepRelativeOffset" false 1.0 1.0 0.0 "/Game/TrackerBot/TrackerBot_Attenuation.TrackerBot_Attenuation" 0)
                    (Collision|SetCollisionEnabled _staticmesh_2 "NoCollision")
                    (Rendering|SetActorHiddenInGame true)
                    (Actor|DestroyActor)))))))))))

(event EventBeginPlay
  (Utilities|FlowControl|Delay 1e+01)
  (Actor|DestroyActor))

(event EventTick
  (params (DeltaSeconds :type Float%20%28single-precision%29))
  (Transformation|AddActorLocalRotation (Math|Rotator|MakeRotator 0.0 0.0 1.0) false false))

(fn ConstructionScript)