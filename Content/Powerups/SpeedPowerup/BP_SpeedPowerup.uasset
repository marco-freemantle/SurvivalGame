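; Spinning speed pickup that temporarily doubles the walk speed of a BP_Demolition character that overlaps it.
; On overlap it raises MaxWalkSpeed, plays an attached sound, disables mesh collision and hides itself, then restores fixed normal speed after a delay.
; Server-named events repeat each speed change on the stored CharacterMovement.
; The actor is never destroyed or re-enabled, and the OnRep handler calls ChangePlayerSpeed with zero speed and no movement component.
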(event OnComponentBeginOverlap(StaticMesh)
  (params (OverlappedComponent :type Primitive%20Component%20Object%20Reference) (OtherActor :type Actor%20Object%20Reference) (OtherComp :type Primitive%20Component%20Object%20Reference) (OtherBodyIndex :type Integer) (bFromSweep :type Boolean) (SweepResult :type Hit%20Result%20Structure%20%28by%20ref%29))
  (bind _staticmesh (Variables|Default|GetStaticMesh))
  (bind _asbp_demolition (Utilities|Casting|CastToBP_Demolition OtherActor))
  (Variables|Default|SetCharacter%20Movement (Variables|/Script/Engine.Character|GetCharacterMovement _asbp_demolition))
  (Variables|/Script/Engine.CharacterMovementComponent|SetMaxWalkSpeed (Variables|/Script/Engine.Character|GetCharacterMovement _asbp_demolition) 1.2e+03)
  (CallFunction|ServerIncreaseSpeed)
  (Audio|SpawnSoundAttached "/Game/Powerups/Pickup-Sound_Cue.Pickup-Sound_Cue" _staticmesh "None" "0, 0, 0" "0, 0, 0" "KeepRelativeOffset" false 1.0 1.0 0.0 "/Game/TrackerBot/TrackerBot_Attenuation.TrackerBot_Attenuation" 0)
  (Collision|SetCollisionEnabled _staticmesh "NoCollision")
  (Rendering|SetActorHiddenInGame true)
  (Utilities|FlowControl|Delay 5.0)
  (Variables|/Script/Engine.CharacterMovementComponent|SetMaxWalkSpeed (Variables|Default|GetCharacter%20Movement) 6e+02)
  (CallFunction|ServerDecreaseSpeed))

(event Custom|ServerIncreaseSpeed
  (Variables|/Script/Engine.CharacterMovementComponent|SetMaxWalkSpeed (Variables|Default|GetCharacter%20Movement) 1.2e+03))

(event Custom|ServerDecreaseSpeed
  (Variables|/Script/Engine.CharacterMovementComponent|SetMaxWalkSpeed (Variables|Default|GetCharacter%20Movement) 6e+02))

(event EventTick
  (params (DeltaSeconds :type Float%20%28single-precision%29))
  (Transformation|AddActorLocalRotation (Math|Rotator|MakeRotator 0.0 0.0 1.0) false false))

(fn ConstructionScript)

(fn OnRepVarMaxWalkSpeed
  (CallFunction|ChangePlayerSpeed 0 0.0))

(fn ChangePlayerSpeed
  (params (Character%20Movement :type Character%20Movement%20Component%20Object%20Reference) (MaxWalkSpeed :type Float%20%28single-precision%29))
  (Variables|/Script/Engine.CharacterMovementComponent|SetMaxWalkSpeed Character%20Movement MaxWalkSpeed))