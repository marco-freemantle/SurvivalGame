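; Grenade launcher projectile that explodes on hitting an SCharacter or when a two-second fuse started at BeginPlay runs out.
; Hits on anything else are ignored.
; Both triggers call ExplodeMulticast, which spawns the explosion effect, applies radial damage credited to the instigator's controller, plays an attenuated sound and destroys the actor.
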(event Custom|ExplodeMulticast
  (bind _returnvalue (Transformation|GetActorLocation))
  (Effects|SpawnEmitteratLocation "/Game/WeaponEffects/Explosion/P_Explosion.P_Explosion" _returnvalue)
  (Game|Damage|ApplyRadialDamage 1e+02 _returnvalue (Variables|Default|GetDamage%20Radius) 0 0 self (Game|GetInstigatorController) false "ECC_Visibility")
  (Audio|SpawnSoundAttached "/Game/TrackerBot/Explosion01_Cue.Explosion01_Cue" (Variables|Default|GetSphere) "None" "0, 0, 0" "0, 0, 0" "KeepRelativeOffset" false 1.0 1.0 0.0 "/Game/TrackerBot/TrackerBot_Attenuation.TrackerBot_Attenuation" 0)
  (Actor|DestroyActor))

(event EventBeginPlay
  (Utilities|FlowControl|Delay 2.0)
  (CallFunction|ExplodeMulticast))

(event Collision|EventHit
  (params (MyComp :type Primitive%20Component%20Object%20Reference) (Other :type Actor%20Object%20Reference) (OtherComp :type Primitive%20Component%20Object%20Reference) (bSelfMoved :type Boolean) (HitLocation :type Vector :default "0, 0, 0") (HitNormal :type Vector :default "0, 0, 0") (NormalImpulse :type Vector :default "0, 0, 0") (Hit :type Hit%20Result%20Structure%20%28by%20ref%29))
  (Utilities|Casting|CastToSCharacter Other)
  (CallFunction|ExplodeMulticast))

(fn ConstructionScript)