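; Explosive mine that detonates once when its health reaches zero, damaging itself when an AdvancedAI or TrackerBot overlaps its box collision.
; Detonation fires a radial force impulse and applies radial damage over the same radius, credited to the health change's instigator.
; Exploded material and explosion effect are set as RepNotify variables, whose OnRep functions swap the mesh material and spawn the particles and sound.
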(event OnHealthChanged(SHealth)
  (params (InHealthComp :type S%20Health%20Component%20Object%20Reference) (Health :type Float%20%28single-precision%29) (HealthDelta :type Float%20%28single-precision%29) (DamageType :type Damage%20Type%20Object%20Reference) (InstigatedBy :type Controller%20Object%20Reference) (DamageCauser :type Actor%20Object%20Reference))
  (if (<= (Math|Float|Truncate Health) 0)
    (if (not (Variables|Default|GethasExploded))
      (Variables|Default|SethasExploded true)
      (Class|RadialForceComponent|FireImpulse (Variables|Default|GetRadialForce))
      (CallFunction|SetMaterial)
      (CallFunction|CreateParticles)
      (Game|Damage|ApplyRadialDamage 1e+02 (Transformation|GetActorLocation) (Variables|/Script/Engine.RadialForceComponent|GetRadius (Variables|Default|GetRadialForce)) 0 0 0 InstigatedBy false "ECC_Visibility"))))

(event OnComponentBeginOverlap(BoxCollision)
  (params (OverlappedComponent :type Primitive%20Component%20Object%20Reference) (OtherActor :type Actor%20Object%20Reference) (OtherComp :type Primitive%20Component%20Object%20Reference) (OtherBodyIndex :type Integer) (bFromSweep :type Boolean) (SweepResult :type Hit%20Result%20Structure%20%28by%20ref%29))
  (Utilities|Casting|CastToBP_AdvancedAI OtherActor
    (:then
      _)
    (:CastFailed
      (Utilities|Casting|CastToSTrackerBot OtherActor)))
  (Game|Damage|ApplyDamage self 1e+02 0 0))

(event Custom|SetMaterial
  ;[1 1 1] Netcode replicating material
  (Variables|Default|SetMaterial_0 "/Game/Enviroment/ExplosiveBarrel/M_ExplosiveBarrelExploded.M_ExplosiveBarrelExploded"))

(event Custom|CreateParticles
  ;[1 1 1] Netcode replicating explosion
  (Variables|Default|SetExplosion%20FX "/Game/Realistic_VFX/Particles/Explosion/P_Explosion_Big_A.P_Explosion_Big_A"))

(fn ConstructionScript)

(fn OnRepMaterial0
  (Rendering|Material|SetMaterial (Variables|Default|GetStaticMesh) 0 (Variables|Default|GetMaterial_0)))

(fn OnRepExplosionFX
  (Effects|SpawnEmitteratLocation (Variables|Default|GetExplosion%20FX) (Transformation|GetActorLocation) "0, 0, 0" "2.000000,2.000000,2.000000")
  (Audio|SpawnSoundAttached "/Game/TrackerBot/Explosion01_Cue.Explosion01_Cue" (Variables|Default|GetStaticMesh) "None" "0, 0, 0" "0, 0, 0" "KeepRelativeOffset" false 1.0 1.0 0.0 0 0))