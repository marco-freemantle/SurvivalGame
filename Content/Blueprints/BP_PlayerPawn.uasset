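; BP_PlayerPawn is a player pawn with a CharacterMovement component that sets up on-screen UI and shows a movement speed debug readout.
; On BeginPlay it creates the WBP_Crosshair and WBP_UI widgets and adds each valid one to the viewport.
; Every Tick it prints MaxWalkSpeed with zero duration, giving a live display of the configured speed limit rather than actual velocity.
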(event EventBeginPlay
  (Utilities|FlowControl|Sequence
    (:then_0
      (bind _returnvalue (UserInterface|CreateWidget "/Game/UI/WBP_Crosshair.WBP_Crosshair_C"))
      (Utilities|IsValid _returnvalue
        (:Is%20Valid
          (UserInterface|Viewport|AddtoViewport _returnvalue 0))))
    (:then_1
      (bind _returnvalue_2 (UserInterface|CreateWidget "/Game/UI/WBP_UI.WBP_UI_C"))
      (Utilities|IsValid _returnvalue_2
        (:Is%20Valid
          (UserInterface|Viewport|AddtoViewport _returnvalue_2 0))))))

(event EventTick
  (params (DeltaSeconds :type Float%20%28single-precision%29))
  (Development|PrintString (Utilities|String|ToString(Float) (Variables|/Script/Engine.CharacterMovementComponent|GetMaxWalkSpeed (Variables|Character|GetCharacterMovement))) true true "(R=0.000000,G=0.660000,B=1.000000,A=1.000000)" 0.0))

(fn ConstructionScript)