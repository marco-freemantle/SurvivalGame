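; Main player character Blueprint that creates the crosshair and main HUD, triggers purchases with E, and deploys abilities.
; UseAbility calls server-named events to spawn the deployable class just ahead along the control rotation, destroying the oldest once the owned limit is reached.
; Boolean gates and an event timer enforce the cooldown between placements, with Tick storing the remaining time.
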(event Custom|ServerSpawnActor_Main
  (bind _abilitiesowned (Variables|Default|GetAbilitiesOwned))
  (if (Variables|Default|GetbCanPlaceAbility)
    (Variables|Default|SetbCanPlaceAbility false)
    (if (< (Utilities|Array|Length (Variables|Default|GetAbilitiesOwned)) (Variables|Default|GetHowManyAbilitesCanBePlaced))
      _
      (else
        (Actor|DestroyActor (Utilities|Array|Get(acopy) _abilitiesowned))
        (Utilities|Array|RemoveIndex _abilitiesowned)))
    (bind _returnvalue (Game|SpawnActorfromClass (Variables|Default|GetDeployableAbility) (Math|Transform|MakeTransform (+ (Transformation|GetActorLocation) (* (Math|Vector|GetForwardVector (Pawn|GetControlRotation (Pawn|GetController) :!class /Script/Engine.Controller)) 1e+02))) "AlwaysSpawn" 0 0))
    (Utilities|Array|Add (Variables|Default|GetAbilitiesOwned) _returnvalue)))

(event Custom|SetBooleanMain
  (CallFunction|SetBooleansTrueServerMain))

(event Custom|SetBooleanFalseServer_Main
  (Variables|Default|SetbCanStartTimer false))

(event Custom|SetBooleansTrueServer_Main
  (Variables|Default|SetbCanPlaceAbility true)
  (Variables|Default|SetbCanStartTimer true))

(event EventBeginPlay
  (Input|SetInputModeGameOnly (Game|GetPlayerController 0))
  (Utilities|FlowControl|Sequence
    (:then_0
      (bind _returnvalue (UserInterface|CreateWidget "/Game/UI/WBP_Crosshair.WBP_Crosshair_C"))
      (Utilities|IsValid _returnvalue
        (:Is%20Valid
          (UserInterface|Viewport|AddtoViewport _returnvalue 0))))
    (:then_1
      (bind _returnvalue_2 (UserInterface|CreateWidget "/Game/UI/WBP_UI_Main.WBP_UI_Main_C"))
      (bind _output_get (Variables|Default|SetUI%20Widget _returnvalue_2))
      (Utilities|IsValid _output_get
        (:Is%20Valid
          (UserInterface|Viewport|AddtoViewport _returnvalue_2 0))))))

(event EventUseAbility
  (if (Utilities|IsValidClass (Variables|Default|GetDeployableAbility))
    (CallFunction|ServerSpawnActorMain)
    (if (Variables|Default|GetbCanStartTimer)
      (CallFunction|SetBooleanFalseServerMain)
      (bind _returnvalue (Utilities|Time|SetTimerbyEvent (delegate Custom|SetBooleanMain) (Variables|Default|GetHowLongBetweenAbilityPlace))))))

(event EventTick
  (params (DeltaSeconds :type Float%20%28single-precision%29))
  (Variables|Default|SetTimeLeftOnAbility (Utilities|Time|GetTimerRemainingTimebyHandle (stale EventUseAbility _returnvalue))))

(event Input|KeyboardEvents|E
  (params (Key :type Key%20Structure))
  (:Pressed
    (Default|CallPurchase)))

(fn ConstructionScript)