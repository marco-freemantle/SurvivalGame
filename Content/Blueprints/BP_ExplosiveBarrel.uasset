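; Explosive barrel actor that detonates once when its SHealth component reports health at or below zero.
; Detonation fires the RadialForce impulse and applies radial damage over the same radius, crediting the instigator that depleted its health.
; The exploded material and explosion particle are stored in RepNotify variables, whose OnRep functions update the mesh and spawn the emitter so the visuals replicate across the network.
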(event OnHealthChanged(SHealth)
  (params (InHealthComp :type S%20Health%20Component%20Object%20Reference) (Health :type Float%20%28single-precision%29) (HealthDelta :type Float%20%28single-precision%29) (DamageType :type Damage%20Type%20Object%20Reference) (InstigatedBy :type Controller%20Object%20Reference) (DamageCauser :type Actor%20Object%20Reference))
  (if (<= (Math|Float|Truncate Health) 0)
    (if (not (Variables|Default|GethasExploded))
      (Variables|Default|SethasExploded true)
      (Class|RadialForceComponent|FireImpulse (Variables|Default|GetRadialForce))
      (CallFunction|SetMaterial)
      (CallFunction|CreateParticles)
      (Game|Damage|ApplyRadialDamage 1e+02 (Transformation|GetActorLocation) (Variables|/Script/Engine.RadialForceComponent|GetRadius (Variables|Default|GetRadialForce)) 0 0 0 InstigatedBy false "ECC_Visibility"))))

(event Custom|SetMaterial
  ;[1 1 1] Netcode replicating material
  (Variables|Default|SetMaterial_0 "/Game/Enviroment/ExplosiveBarrel/M_ExplosiveBarrelExploded.M_ExplosiveBarrelExploded"))

(event Custom|CreateParticles
  ;[1 1 1] Netcode replicating explosion
  (Variables|Default|SetExplosion%20FX "/Game/Realistic_VFX/Particles/Explosion/P_Explosion_Big_A.P_Explosion_Big_A"))

(fn ConstructionScript)

(fn OnRepMaterial0
  (Rendering|Material|SetMaterial (Variables|Default|GetStaticMesh) 0 (Variables|Default|GetMaterial_0)))

(fn OnRepExplosionFX
  (Effects|SpawnEmitteratLocation (Variables|Default|GetExplosion%20FX) (Transformation|GetActorLocation) "0, 0, 0" "2.000000,2.000000,2.000000"))