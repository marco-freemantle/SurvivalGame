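; BP_Demolition is a player class, apparently a demolition character, that deploys barrels as its ability and adds crosshair and UI widgets on BeginPlay.
; UseAbility calls ServerSpawnActor, which spawns the DeployableAbility class just ahead of the controller's aim.
; BarrelsOwned caps live barrels by destroying the oldest, and a timer-reset flag enforces a short placement cooldown.
; Tick prints the barrel count for debugging.
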(event Custom|ServerSpawnActor
  (bind _barrelsowned (Variables|Default|GetBarrelsOwned))
  (if (Variables|Default|GetbCanPlaceBarrel)
    (if (< (Utilities|Array|Length (Variables|Default|GetBarrelsOwned)) 5)
      _
      (else
        (Actor|DestroyActor (Utilities|Array|Get(acopy) _barrelsowned))
        (Utilities|Array|RemoveIndex _barrelsowned)))
    (bind _returnvalue (Game|SpawnActorfromClass (Variables|Default|GetDeployableAbility) (Math|Transform|MakeTransform (+ (Transformation|GetActorLocation) (* (Math|Vector|GetForwardVector (Pawn|GetControlRotation (Pawn|GetController) :!class /Script/Engine.Controller)) 1e+02))) "AlwaysSpawn" 0 0))
    (Utilities|Array|Add (Variables|Default|GetBarrelsOwned) _returnvalue)
    (Variables|Default|SetbCanPlaceBarrel false)
    (Utilities|Time|SetTimerbyEvent (delegate Custom|SetBoolean) 1.0)))

(event Custom|SetBoolean
  (Variables|Default|SetbCanPlaceBarrel true))

(event EventBeginPlay
  (Utilities|FlowControl|Sequence
    (:then_0
      (bind _returnvalue (UserInterface|CreateWidget "/Game/UI/WBP_Crosshair.WBP_Crosshair_C"))
      (Utilities|IsValid _returnvalue
        (:Is%20Valid
          (UserInterface|Viewport|AddtoViewport _returnvalue 0))))
    (:then_1
      (bind _returnvalue_2 (UserInterface|CreateWidget "/Game/UI/WBP_UI.WBP_UI_C"))
      (Utilities|IsValid _returnvalue_2
        (:Is%20Valid
          (UserInterface|Viewport|AddtoViewport _returnvalue_2 0))))))

(event EventUseAbility
  (if (Utilities|IsValidClass (Variables|Default|GetDeployableAbility))
    (CallFunction|ServerSpawnActor)))

(event EventTick
  (params (DeltaSeconds :type Float%20%28single-precision%29))
  (Development|PrintString (Utilities|String|ToString(Integer) (Utilities|Array|Length (Variables|Default|GetBarrelsOwned))) true true "(R=0.000000,G=0.660000,B=1.000000,A=1.000000)" 0.0))

(fn ConstructionScript)