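; BP_HealingAbility is a healing area that periodically restores health to team 0 actors inside its overlap sphere.
; Any overlap begin calls ServerHealPlayers, which sets a looping one-second timer on Heal Players; nothing clears it.
; Each tick, Heal Players queries the sphere's overlapping actors and adds a fixed amount of health through each valid SHealthComponent whose TeamNum is 0.
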(event OnComponentBeginOverlap(SphereOverlap)
  (params (OverlappedComponent :type Primitive%20Component%20Object%20Reference) (OtherActor :type Actor%20Object%20Reference) (OtherComp :type Primitive%20Component%20Object%20Reference) (OtherBodyIndex :type Integer) (bFromSweep :type Boolean) (SweepResult :type Hit%20Result%20Structure%20%28by%20ref%29))
  (CallFunction|ServerHealPlayers))

(event Custom|ServerHealPlayers
  (Utilities|Time|SetTimerbyFunctionName 0 "Heal Players" 1.0 true))

(fn ConstructionScript)

(fn HealPlayers
  (for _array_element (Collision|GetOverlappingActors (Variables|Default|GetSphereOverlap) 0 :!class /Script/Engine.PrimitiveComponent)
    (Utilities|IsValid (Actor|GetComponentbyClass _array_element "/Script/Survival.SHealthComponent")
      (:Is%20Valid
        (if (== (Variables|/Script/Survival.SHealthComponent|GetTeamNum (Actor|GetComponentbyClass _array_element "/Script/Survival.SHealthComponent")) 0)
          (Class|SHealthComponent|AddHealth (Actor|GetComponentbyClass _array_element "/Script/Survival.SHealthComponent") 1e+01))))))