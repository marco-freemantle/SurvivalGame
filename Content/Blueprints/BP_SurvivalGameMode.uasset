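; Survival game mode that spawns AI enemies and bosses, scores kills and spawns each player as their chosen character class.
; SpawnNewBot and SpawnBoss run an EQS location query, spawning a random advanced AI or tracker bot, or a boss, at returned locations.
; An actor-killed binding adjusts the killer's player-state score, penalizing main-character kills and rewarding other pawn kills.
; SpawnDefaultPawnFor takes the pawn class from the player controller.
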(event Custom|OnQueryFinishedEvent_Event_1
  (params (QueryInstance :type Env%20Query%20Instance%20Blueprint%20Wrapper%20Object%20Reference) (QueryStatus :type EEnvQueryStatus%20Enum :default "Processing"))
  (switch Utilities|FlowControl|Switch|SwitchonEEnvQueryStatus QueryStatus
    (:Success
      (bind _resultlocations (AI|EQS|GetQueryResultsasLocations QueryInstance))
      (for _array_element _resultlocations
        (Game|SpawnActorfromClass "/Game/AdvancedAI/BP_Boss.BP_Boss_C" (Math|Transform|MakeTransform _array_element) "AdjustIfPossibleButDontSpawnIfColliding" 0 0)))))

(event Custom|OnActorKilledEvent
  (params (VictimActor :type Actor%20Object%20Reference) (KillerActor :type Actor%20Object%20Reference) (KillerController :type Controller%20Object%20Reference))
  (bind _returnvalue (Pawn|GetControlledPawn KillerController))
  (bind _playerstate (Variables|/Script/Engine.Pawn|GetPlayerState _returnvalue))
  (bind _aspawn (Utilities|Casting|CastToPawn VictimActor))
  (Utilities|Casting|CastToBP_MainCharacter _aspawn
    (:then
      (Utilities|IsValid KillerController
        (:Is%20Valid
          (bind _assplayer_state (Utilities|Casting|CastToSPlayerState _playerstate))
          (Class|SPlayerState|TakeAwayScore _assplayer_state 5e+02))))
    (:CastFailed
      (Utilities|IsValid KillerController
        (:Is%20Valid
          (bind _assplayer_state_2 (Utilities|Casting|CastToSPlayerState _playerstate))
          (Class|SPlayerState|AddScore _assplayer_state_2 2e+01))))))

(event Custom|OnQueryFinishedEvent_Event_0
  (params (QueryInstance :type Env%20Query%20Instance%20Blueprint%20Wrapper%20Object%20Reference) (QueryStatus :type EEnvQueryStatus%20Enum :default "Processing"))
  (switch Utilities|FlowControl|Switch|SwitchonEEnvQueryStatus QueryStatus
    (:Success
      (bind _resultlocations (AI|EQS|GetQueryResultsasLocations QueryInstance))
      (for _array_element _resultlocations
        (Game|SpawnActorfromClass (select (<= (Math|Random|RandomFloatinRange 0.0 1e+02) 45.0) "/Game/AdvancedAI/BP_AdvancedAI.BP_AdvancedAI_C" "/Game/TrackerBot/BP_TrackerBot.BP_TrackerBot_C") (Math|Transform|MakeTransform _array_element) "AdjustIfPossibleButDontSpawnIfColliding" 0 0)))))

(event EventSpawnBoss
  (bind _returnvalue (AI|EQS|RunEQSQuery "/Game/Blueprints/EQS_FindSpawnLocatoin.EQS_FindSpawnLocatoin" self "RandomBest25Pct"))
  (EventDispatchers|AssignOnQueryFinishedEvent _returnvalue (delegate Custom|OnQueryFinishedEvent_Event_1)))

(event EventSpawnNewBot
  (bind _returnvalue (AI|EQS|RunEQSQuery "/Game/Blueprints/EQS_FindSpawnLocatoin.EQS_FindSpawnLocatoin" self "RandomBest25Pct"))
  (EventDispatchers|AssignOnQueryFinishedEvent _returnvalue (delegate Custom|OnQueryFinishedEvent_Event_0)))

(event EventHandleStartingNewPlayer
  (params (NewPlayer :type Player%20Controller%20Object%20Reference))
  (Class|GameModeBase|RestartPlayeratPlayerStart NewPlayer (Class|GameModeBase|FindPlayerStart NewPlayer)))

(event EventBeginPlay
  (EventDispatchers|BindEventtoOnActorKilled (delegate Custom|OnActorKilledEvent)))

(fn ConstructionScript)

(fn SpawnDefaultPawnfor
  (params (NewPlayer :type Controller%20Object%20Reference) (StartSpot :type Actor%20Object%20Reference))
  (bind _asbp_player_controller (Utilities|Casting|CastToBP_PlayerController NewPlayer))
  (Default|GetCharacterClass _asbp_player_controller)
  (bind _returnvalue (Game|SpawnActorfromClass (Variables|/Game/Blueprints/BP_PlayerController.BP_PlayerController_C|GetChosen%20Class _asbp_player_controller) (Transformation|GetActorTransform StartSpot) "Undefined" 0 0))
  (return _returnvalue))