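; Tank Blueprint with a deployable ability that spawns a configurable actor class in front of the controller's aim.
; UseAbility calls server-named events to spawn the deployable and starts a cooldown timer that re-enables placement, with Tick tracking the time left.
; An owned-actor array caps placements by destroying the oldest, and each spawn also schedules removal after a delay.
; The construction script sets the placement limit and cooldown length.
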(event Custom|ServerSpawnActor_Tank
  (bind _abilitiesowned (Variables|Default|GetAbilitiesOwned))
  (if (Variables|Default|GetbCanPlaceAbility)
    (Variables|Default|SetbCanPlaceAbility false)
    (if (< (Utilities|Array|Length (Variables|Default|GetAbilitiesOwned)) (Variables|Default|GetHowManyAbilitesCanBePlaced))
      _
      (else
        (Actor|DestroyActor (Utilities|Array|Get(acopy) _abilitiesowned))
        (Utilities|Array|RemoveIndex _abilitiesowned)))
    (bind _returnvalue (Game|SpawnActorfromClass (Variables|Default|GetDeployableAbility) (Math|Transform|MakeTransform (+ (Transformation|GetActorLocation) (* (Math|Vector|GetForwardVector (Pawn|GetControlRotation (Pawn|GetController) :!class /Script/Engine.Controller)) 1e+02))) "AlwaysSpawn" 0 0))
    (Utilities|Array|Add (Variables|Default|GetAbilitiesOwned) _returnvalue)
    (Utilities|FlowControl|Delay 1e+01)
    (Actor|DestroyActor _returnvalue)
    (Utilities|Array|RemoveIndex (Variables|Default|GetAbilitiesOwned))))

(event Custom|SetBooleanSupport
  (CallFunction|SetBooleansTrueServerTank))

(event Custom|SetBooleanFalseServer_Tank
  (Variables|Default|SetbCanStartTimer false))

(event Custom|SetBooleansTrueServer_Tank
  (Variables|Default|SetbCanPlaceAbility true)
  (Variables|Default|SetbCanStartTimer true))

(event EventBeginPlay
  (|CallParentFunction) ; This node is disabled and will not be called.\nDrag off pins to build functionality.
)

(event EventUseAbility
  (if (Utilities|IsValidClass (Variables|Default|GetDeployableAbility))
    (CallFunction|ServerSpawnActorTank)
    (if (Variables|Default|GetbCanStartTimer)
      (CallFunction|SetBooleanFalseServerTank)
      (bind _returnvalue (Utilities|Time|SetTimerbyEvent (delegate Custom|SetBooleanSupport) (Variables|Default|GetHowLongBetweenAbilityPlace))))))

(event EventTick
  (params (DeltaSeconds :type Float%20%28single-precision%29))
  (Variables|Default|SetTimeLeftOnAbility (Utilities|Time|GetTimerRemainingTimebyHandle (stale EventUseAbility _returnvalue))))

(fn ConstructionScript
  (|CallParentFunction)
  (Variables|Default|SetHowManyAbilitesCanBePlaced 1)
  (Variables|Default|SetHowLongBetweenAbilityPlace 2e+01))