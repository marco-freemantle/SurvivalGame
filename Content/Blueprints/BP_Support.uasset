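; Support character Blueprint whose ability spawns a deployable, attached to the mesh's HealPointSocket, with a fireflies particle effect.
; UseAbility calls server-named events to spawn it and starts a cooldown timer that re-enables placement, with Tick tracking time left.
; The spawn evicts the oldest deployable at the limit, triggers SpawnParticlesMulticast, then after a fixed delay destroys the deployable and a particle component.
; The construction script sets limit and cooldown.
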(event Custom|ServerSpawnActor_Support
  (bind _abilitiesowned (Variables|Default|GetAbilitiesOwned))
  (if (Variables|Default|GetbCanPlaceAbility)
    (Variables|Default|SetbCanPlaceAbility false)
    (if (< (Utilities|Array|Length (Variables|Default|GetAbilitiesOwned)) (Variables|Default|GetHowManyAbilitesCanBePlaced))
      _
      (else
        (Actor|DestroyActor (Utilities|Array|Get(acopy) _abilitiesowned))
        (Utilities|Array|RemoveIndex _abilitiesowned)))
    (bind _returnvalue (Game|SpawnActorfromClass (Variables|Default|GetDeployableAbility) (Math|Transform|MakeTransform (Transformation|GetActorLocation) "0, 0, 0" "0.030000,0.030000,0.030000") "AlwaysSpawn" 0 0))
    (Utilities|Array|Add (Variables|Default|GetAbilitiesOwned) _returnvalue)
    (Transformation|AttachComponentToComponent _returnvalue (Variables|Character|GetMesh) "HealPointSocket" "SnapToTarget" "SnapToTarget" "KeepRelative" true)
    (CallFunction|SpawnParticlesMulticast)
    (Utilities|FlowControl|Delay 1e+01)
    (Actor|DestroyActor _returnvalue)
    (Utilities|Array|RemoveIndex (Variables|Default|GetAbilitiesOwned))
    (CallFunction|DestroyEmitter)))

(event Custom|SetBooleanSupport
  (CallFunction|SetBooleansTrueServerSupport))

(event Custom|SetBooleanFalseServer_Support
  (Variables|Default|SetbCanStartTimer false))

(event Custom|SetBooleansTrueServer_Support
  (Variables|Default|SetbCanPlaceAbility true)
  (Variables|Default|SetbCanStartTimer true))

(event Custom|Destroy%20Emitter
  (bind _returnvalue (Actor|GetComponentbyClass "/Script/Engine.ParticleSystemComponent"))
  (Utilities|IsValid _returnvalue
    (:Is%20Valid
      (Components|DestroyComponent _returnvalue))))

(event Custom|SpawnParticlesMulticast
  (bind _returnvalue (Effects|SpawnEmitterAttached (Variables|Default|GetFireflies%20Particles) (Variables|Default|GetCapsuleComponent) "HealPointSocket" "0.000000,0.000000,-300.000000" "0, 0, 0" "1.000000,1.000000,1.000000" "SnapToTarget"))
  (Variables|Default|SetHealingEmitterSpawned _returnvalue))

(event EventBeginPlay
  (|CallParentFunction) ; This node is disabled and will not be called.\nDrag off pins to build functionality.
)

(event EventUseAbility
  (if (Utilities|IsValidClass (Variables|Default|GetDeployableAbility))
    (CallFunction|ServerSpawnActorSupport)
    (if (Variables|Default|GetbCanStartTimer)
      (CallFunction|SetBooleanFalseServerSupport)
      (bind _returnvalue (Utilities|Time|SetTimerbyEvent (delegate Custom|SetBooleanSupport) (Variables|Default|GetHowLongBetweenAbilityPlace))))))

(event EventTick
  (params (DeltaSeconds :type Float%20%28single-precision%29))
  (Variables|Default|SetTimeLeftOnAbility (Utilities|Time|GetTimerRemainingTimebyHandle (stale EventUseAbility _returnvalue))))

(event Collision|EventActorBeginOverlap
  (params (OtherActor :type Actor%20Object%20Reference)))

(fn ConstructionScript
  (|CallParentFunction)
  (Variables|Default|SetHowManyAbilitesCanBePlaced 1)
  (Variables|Default|SetHowLongBetweenAbilityPlace 2e+01))