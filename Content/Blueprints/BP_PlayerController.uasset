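; BP_PlayerController is the player controller for what appears to be an online survival game, handling respawn requests, menu return and audio transitions.
; GetCharacterClass reads the chosen class from OnlineGameInstance and passes it to RequestRespawn, which asks BP_SurvivalGameMode to respawn this player only when running with authority.
; Other events stop menu music and start ambient sound through the game instance, or open the main menu level when leaving a session.
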(event Custom|GetCharacterClass
  (bind _asonline_game_instance (Utilities|Casting|CastToOnlineGameInstance (Game|GetGameInstance)))
  (bind _output_get (Variables|Default|SetChosen%20Class (Variables|/Game/Menus/OnlineMenuSystem/OnlineGameInstance.OnlineGameInstance_C|GetChosenClass _asonline_game_instance)))
  (CallFunction|RequestRespawn _output_get))

(event Custom|LeaveSessionInProgress
  (Game|OpenLevel(byObjectReference) "/Game/Menus/OnlineMenuSystem/MainMenu.MainMenu"))

(event Custom|RequestRespawn
  (params (Chosen%20Class :type BP%20Main%20Character%20Class%20Reference))
  (Networking|SwitchHasAuthority
    (:Authority
      (bind _asbp_survival_game_mode (Utilities|Casting|CastToBP_SurvivalGameMode (Game|GetGameMode)))
      (Default|Respawn _asbp_survival_game_mode self Chosen%20Class))))

(event Custom|StopMenuMusic
  (bind _asonline_game_instance (Utilities|Casting|CastToOnlineGameInstance (Game|GetGameInstance)))
  (Default|StopMenuAudio _asonline_game_instance))

(event Custom|StartAmbientAudio
  (bind _asonline_game_instance (Utilities|Casting|CastToOnlineGameInstance (Game|GetGameInstance)))
  (Default|PlayGameAmbientSound _asonline_game_instance))

(fn ConstructionScript)